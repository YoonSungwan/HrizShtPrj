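; BP_Map3 is a map actor that slides along a direction until it reaches a stopping point.
; Each Tick, while not stopped, it moves by Dir scaled by MoveSpeed and delta time, without sweep.
; Once its world Y drops to a hardcoded threshold of -160 or lower, it sets the Stoped flag and stays in place.
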(event EventBeginPlay)

(event EventTick
  (params (DeltaSeconds :type Float%20%28single-precision%29))
  (if (not (Variables|Default|GetbStoped))
    (Transformation|SetActorLocation (+ (Transformation|GetActorLocation) (* (Variables|Default|GetDir) (Variables|Default|GetMoveSpeed) DeltaSeconds)) false false)
    (if (<= (.y (Transformation|GetActorLocation)) -1.6e+02)
      (Variables|Default|SetbStoped true))))

(fn ConstructionScript)