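; BP_SelectGameModeBase is a game mode, apparently for a selection screen, that slides a camera actor between positions.
; StartMovement calls UpdateTargetLocation, then plays the Animatior timeline to lerp the camera from StartPosition to TargetPosition.
; On finish it snaps the camera to the target, stores that as the next StartPosition and resets the timeline's time for the following move.
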(event Custom|StartMovement
  (bind _cameraactor (Variables|Default|GetCameraActor))
  (Class|SelectGameModeBase|UpdateTargetLocation)
  (bind _lerptime (Timeline|Animatior Play)
    (:Update
      (Transformation|SetActorLocation _cameraactor (Math|Vector|Lerp(Vector) (Variables|Default|GetStartPosition) (Variables|Default|GetTargetPosition) _lerptime) false false))
    (:Finished
      (Transformation|SetActorLocation _cameraactor (Variables|Default|GetTargetPosition) false false)
      (Variables|Default|SetStartPosition (Variables|Default|GetTargetPosition))
      (Timeline|Animatior SetNewTime))))

(event EventBeginPlay
  (|CallParentFunction))

(event EventTick
  (params (DeltaSeconds :type Float%20%28single-precision%29)))

(fn ConstructionScript)